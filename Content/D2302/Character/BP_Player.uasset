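; BP_Player is a player Blueprint that provides mouse-drag camera control through its SpringArm.
; Each mouse button stores the cursor's start position and runs a looping timer until released.
; Left drag shifts the socket offset along the dominant axis, accumulating each tick so pan speed grows with distance from the start.
; Right drag sets yaw from the rotation captured on press plus horizontal cursor displacement.
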(event `Key|LeftMouseButton`
  (params (Key :type "Key Structure"))
  (:`Pressed`
    (bind _returnvalue (`WidgetLayoutLibrary.GetMousePositionOnViewport`))
    (set `self.MouseStartLLocation` _returnvalue)
    (bind _returnvalue_2 (`KismetSystemLibrary.K2_SetTimerDelegate` (`|CreateDelegate` :!event `UpdateMouseLLocationEvent`) 0.05 true))
    (set `self.UpdateMouseLLocationTimerHandle` _returnvalue_2))
  (:`Released`
    (`KismetSystemLibrary.K2_ClearAndInvalidateTimerHandle` (`self.UpdateMouseLLocationTimerHandle`))))

(event `UpdateMouseLLocationEvent`
  (bind _springarm (`self.SpringArm`))
  (bind _springarm_2 (`self.SpringArm`))
  (bind (_socketoffset_x _socketoffset_y _socketoffset_z) (`KismetMathLibrary.BreakVector` (`SpringArmComponent.SocketOffset` _springarm)))
  (bind (_socketoffset_x_2 _socketoffset_y_2 _socketoffset_z_2) (`KismetMathLibrary.BreakVector` (`SpringArmComponent.SocketOffset` _springarm_2)))
  (bind _returnvalue (`WidgetLayoutLibrary.GetMousePositionOnViewport`))
  (bind (_returnvalue_x _returnvalue_y) (`KismetMathLibrary.BreakVector2D` (- _returnvalue (`self.MouseStartLLocation`))))
  (if (> (`KismetMathLibrary.Abs` _returnvalue_x) (`KismetMathLibrary.Abs` _returnvalue_y))
    (set `SpringArmComponent.SocketOffset` (`KismetMathLibrary.MakeVector` _socketoffset_x_2 (+ _socketoffset_y_2 (* _returnvalue_x -1.0)) _socketoffset_z_2) _springarm_2)
    (else
      (set `SpringArmComponent.SocketOffset` (`KismetMathLibrary.MakeVector` _socketoffset_x _socketoffset_y (+ _socketoffset_z (* _returnvalue_y 1.0))) _springarm))))

(event `Key|RightMouseButton`
  (params (Key :type "Key Structure"))
  (:`Pressed`
    (bind _returnvalue (`WidgetLayoutLibrary.GetMousePositionOnViewport`))
    (set `self.MouseStartRLocation` _returnvalue)
    (bind _returnvalue_2 (`KismetSystemLibrary.K2_SetTimerDelegate` (`|CreateDelegate` :!event `UpdateMouseRLocationEvent`) 0.05 true))
    (set `self.UpdateMouseRLocationTimerHandle` _returnvalue_2)
    (set `self.MoueseRSpringArmRelativeRotation` (`SceneComponent.RelativeRotation` (`self.SpringArm`))))
  (:`Released`
    (`KismetSystemLibrary.K2_ClearAndInvalidateTimerHandle` (`self.UpdateMouseRLocationTimerHandle`))))

(event `UpdateMouseRLocationEvent`
  (bind (_moueserspringarmrelativerotation_roll _moueserspringarmrelativerotation_pitch _moueserspringarmrelativerotation_yaw) (`KismetMathLibrary.BreakRotator` (`self.MoueseRSpringArmRelativeRotation`)))
  (bind _returnvalue (`WidgetLayoutLibrary.GetMousePositionOnViewport`))
  (bind _returnvalue_x (`KismetMathLibrary.BreakVector2D` (- _returnvalue (`self.MouseStartRLocation`))))
  (`SceneComponent.K2_SetRelativeRotation` (`self.SpringArm`) (`KismetMathLibrary.MakeRotator` _moueserspringarmrelativerotation_roll _moueserspringarmrelativerotation_pitch (+ _moueserspringarmrelativerotation_yaw (* _returnvalue_x 1.0))) false false))

(fn `UserConstructionScript`)