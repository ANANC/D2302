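; Shop shelf actor that displays a row of meshes reflecting the stock of one prop in a named shop.
; Shortly after BeginPlay, SetGoods fetches the prop config, binds to the shop's number-update delegate and shows the current count.
; Each matching update destroys and respawns static mesh components at fixed intervals, with the count capped by ShowGoodNumber.
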(event `self.ReceiveBeginPlay`
  (`KismetSystemLibrary.Delay` 1.0)
  (`self.SetGoods` (`self.ShopName`) (`self.ShopPropName`)))

(event `self.ReceiveDestroyed`)

(fn `SetGoods`
  (params (ShopName :type Name) (ShopPropName :type Name))
  (bind _returnvalue (`GameCommonFunctionLibrary.GetShopInstanceSubsystem`))
  (bind _returnvalue_2 (`ShopInstanceSubsystem.GetShop` _returnvalue (`self.ShopName`)))
  (set `self.ShopName` ShopName)
  (set `self.ShopPropName` ShopPropName)
  (set `self.PropConfig` (`PropInstanceSubsystem.GetPropConfigableInfo` (`GameCommonFunctionLibrary.GetPropInstanceSubsystem`) ShopPropName))
  (`/Engine/EditorBlueprintResources/StandardMacros.IsValid` _returnvalue
    (:`Is Valid`
      (`/Engine/EditorBlueprintResources/StandardMacros.IsValid` _returnvalue_2
        (:`Is Valid`
          (add `BaseShop.ShopPropNumberUpdateDelegate` _returnvalue_2 (`|CreateDelegate` :!event `ShopPropNumberUpdateCallback`))
          (`self.UpdateCurPropNumber` (`BaseShop.GetPropNumber` _returnvalue_2 (`self.ShopPropName`))))))))

(fn `ShopPropNumberUpdateCallback`
  (params (shopName :type Name) (propName :type Name) (number :type Integer) (price :type Integer))
  (if (and (== shopName (`self.ShopName`)) (== propName (`self.ShopPropName`)))
    (`self.UpdateCurPropNumber` number)))

(fn `UpdateCurPropNumber`
  (params (propNumber :type Integer))
  (locals (showNumber :type Integer :default 10) (location :type "Vector Structure"))
  (bind _shownumber (`local.showNumber`))
  (bind (_propconfig_titlename _propconfig_statamesh) (break `PropTableConfigData` (`self.PropConfig`)))
  (`|ExecutionSequence`
    (:`then_0`
      (if (> propNumber (`self.ShowGoodNumber`))
        (set `local.showNumber` (`self.ShowGoodNumber`))
        (else
          (set `local.showNumber` propNumber))))
    (:`then_1`
      (for _array_element (`self.GoodMeshs`)
        (`ActorComponent.K2_DestroyComponent` _array_element))
      (`KismetArrayLibrary.Array_Clear` (`self.GoodMeshs`)))
    (:`then_2`
      (if (> _shownumber 0)
        (for _index (range (+ _shownumber 1))
          (bind _output_get (set `local.location` (+ (`self.InitLocation`) (* _index (`self.GoodInterval`)))))
          (bind _returnvalue (`|AddComponentByClass` "/Script/Engine.StaticMeshComponent" false (`KismetMathLibrary.MakeTransform` _output_get (struct) (`self.InitRotation`))))
          (`KismetArrayLibrary.Array_Add` (`self.GoodMeshs`) _returnvalue)
          (`StaticMeshComponent.SetStaticMesh` _returnvalue _propconfig_statamesh))))))

(fn `UserConstructionScript`)